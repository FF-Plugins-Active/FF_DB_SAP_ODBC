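; Template Blueprint that exercises the SAP ODBC plugin against a SQL test database.
; On BeginPlay it spawns a SAP_ODBC_Manager, initializes the environment and connects with a password read from GI_SplitScreen.
; After a short delay, FQueryView runs a prepared SELECT and prints id/name rows, with color-coded status messages along the way.
; FQueryInsert demonstrates a batched, committed insert but is never called, as are alternative metadata-driven result readers.
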(event EventBeginPlay
  (bind _returnvalue (Game|SpawnActorfromClass "/Script/FF_DB_SAPODBC.SAP_ODBC_Manager" (Math|Transform|MakeTransform "0, 0, 0" "0, 0, 0" "1.000000,1.000000,1.000000") "Undefined" "MultiplyWithRoot" 0 0))
  (bind _output_get (Variables|Default|SetSAP_ODBC_Manager _returnvalue))
  (bind _returnvalue_2 (Class|SAPODBCManager|SAPODBCInitEnvironment _output_get))
  (if _returnvalue_2
    (bind _asgi_split_screen (Utilities|Casting|CastToGI_SplitScreen (Game|GetGameInstance)))
    (bind (_out_code _createdconnection _returnvalue_3) (Class|SAPODBCManager|SAPODBCConnectionCreate (Variables|Default|GetSAP_ODBC_Manager) "VM_SQL_UE5_HS" "vm_sql_ue5" (.Value (Utilities|Map|Find (Variables|/Game/Player/Desktop/GI_SplitScreen.GI_SplitScreen_C|GetPasswords _asgi_split_screen) "odbc")) false))
    (Development|PrintString _out_code true true (Math|Color|SelectColor "(R=0.000000,G=1.000000,B=0.000000,A=1.000000)" "(R=1.000000,G=0.000000,B=0.000000,A=1.000000)" _returnvalue_3) 3e+01)
    (if _returnvalue_3
      (Variables|Default|SetSAP_ODBC_Connection _createdconnection)
      (Utilities|FlowControl|Delay 2.0)
      (CallFunction|FQueryView))))

(fn ConstructionScript)

(fn FQueryInsert
  (bind (_out_code _out_statement _returnvalue) (Class|SAPODBCConnection|PrepareStatement (Variables|Default|GetSAP_ODBC_Connection) (Class|SAPODBCBPLibrary|InsertInto "ue5_test.dbo.Table_1" (Utilities|Set|MakeSet "id" "name"))))
  (Development|PrintString _out_code true true (Math|Color|SelectColor "(R=0.000000,G=1.000000,B=0.000000,A=1.000000)" "(R=1.000000,G=0.000000,B=0.000000,A=1.000000)" _returnvalue) 3e+01)
  (if _returnvalue
    (LocalVariables|SetLOC_Statement _out_statement)
    (Class|SAPODBCStatement|SetInt (LocalVariables|GetLOC_Statement) 3 1)
    (Class|SAPODBCStatement|SetString (LocalVariables|GetLOC_Statement) "Test User" 2)
    (Class|SAPODBCStatement|AddBatch (LocalVariables|GetLOC_Statement))
    (bind _out_code_2 (Class|SAPODBCStatement|ExecuteBatch (LocalVariables|GetLOC_Statement)))
    (Development|PrintString _out_code_2 true true "(R=0.000000,G=0.660000,B=1.000000,A=1.000000)" 3e+01)
    (bind (_out_code_3 _returnvalue_2) (Class|SAPODBCStatement|CommitStatement (LocalVariables|GetLOC_Statement)))
    (Development|PrintString _out_code_3 true true (Math|Color|SelectColor "(R=0.000000,G=1.000000,B=0.000000,A=1.000000)" "(R=1.000000,G=0.000000,B=0.000000,A=1.000000)" _returnvalue_2) 3e+01)
    (return)
    (else
      (return))))

(fn FQueryView
  (bind (_out_code _out_statement _returnvalue) (Class|SAPODBCConnection|PrepareStatement (Variables|Default|GetSAP_ODBC_Connection) "SELECT id, name FROM ue5_test.dbo.Table_1 WHERE id>1"))
  (Development|PrintString _out_code true true (Math|Color|SelectColor "(R=0.000000,G=1.000000,B=0.000000,A=1.000000)" "(R=1.000000,G=0.000000,B=0.000000,A=1.000000)" _returnvalue) 3e+01)
  (if _returnvalue
    (LocalVariables|SetLOC_Statement _out_statement)
    (bind (_out_code_2 _out_result _returnvalue_2) (Class|SAPODBCStatement|ExecuteQuery (LocalVariables|GetLOC_Statement)))
    (Development|PrintString _out_code_2 true true (Math|Color|SelectColor "(R=0.000000,G=1.000000,B=0.000000,A=1.000000)" "(R=1.000000,G=0.000000,B=0.000000,A=1.000000)" _returnvalue_2) 3e+01)
    (if _returnvalue_2
      (LocalVariables|SetLOC_Result _out_result)
      (bind _out_string (Class|SAPODBCResult|GetInt (LocalVariables|GetLOC_Result) 1))
      (LocalVariables|SetArray_IDs _out_string)
      (bind _out_string_2 (Class|SAPODBCResult|GetString (LocalVariables|GetLOC_Result) 2))
      (LocalVariables|SetArray_Names _out_string_2)
      (for (_array_element _array_index) (LocalVariables|GetArray_IDs)
        (Development|PrintString (Utilities|String|Append "ID = " (Utilities|String|ToString(Integer) _array_element) " // " "NAME = " (Utilities|Array|Get(acopy) (LocalVariables|GetArray_Names) _array_index)) true true "(R=0.000000,G=0.660000,B=1.000000,A=1.000000)" 3e+01))
      (return)
      (else
        (return)))
    (else
      (return))))