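; Template Blueprint that demonstrates writing to a SQL database through the SAP ODBC plugin.
; On BeginPlay it spawns the ODBC manager, initializes the environment, opens a connection with hardcoded credentials, then waits briefly before inserting.
; The insert function prepares a parameterized statement, binds a test row, executes it as a batch and commits.
; On-screen prints report each step, with connect, prepare and commit color-coded by success.
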(event EventBeginPlay
  (bind _returnvalue (Game|SpawnActorfromClass "/Script/FF_DB_SAPODBC.SAP_ODBC_Manager" (Math|Transform|MakeTransform "0, 0, 0" "0, 0, 0" "1.000000,1.000000,1.000000") "Undefined" "MultiplyWithRoot" 0 0))
  (bind _output_get (Variables|Default|SetSAP_ODBC_Manager _returnvalue))
  (bind _returnvalue_2 (Class|SAPODBCManager|SAPODBCInitEnvironment _output_get))
  (if _returnvalue_2
    (bind (_out_code _createdconnection _returnvalue_3) (Class|SAPODBCManager|SAPODBCCreateConnection (Variables|Default|GetSAP_ODBC_Manager) "vm_sql_ue5" "vm_sql_ue5" "37296937" false))
    (Development|PrintString _out_code true true (Math|Color|SelectColor "(R=0.000000,G=1.000000,B=0.000000,A=1.000000)" "(R=1.000000,G=0.000000,B=0.000000,A=1.000000)" _returnvalue_3) 3e+01)
    (if _returnvalue_3
      (Variables|Default|SetSAP_ODBC_Connection _createdconnection)
      (Utilities|FlowControl|Delay 2.0)
      (CallFunction|FSendQueryInsert))))

(fn ConstructionScript)

(fn FSendQueryInsert
  (bind (_out_code _out_statement _returnvalue) (Class|SAPODBCConnection|PrepareStatement (Variables|Default|GetSAP_ODBC_Connection) (Class|SAPODBCBPLibrary|InsertInto "ue5_test.dbo.Table_1" (Utilities|Set|MakeSet "id" "name"))))
  (Development|PrintString _out_code true true (Math|Color|SelectColor "(R=0.000000,G=1.000000,B=0.000000,A=1.000000)" "(R=1.000000,G=0.000000,B=0.000000,A=1.000000)" _returnvalue) 3e+01)
  (if _returnvalue
    (LocalVariables|SetLOC_Statement _out_statement)
    (Class|SAPODBCStatement|SetInt (LocalVariables|GetLOC_Statement) 3 1)
    (Class|SAPODBCStatement|SetString (LocalVariables|GetLOC_Statement) "Test User" 2)
    (Class|SAPODBCStatement|AddBatch (LocalVariables|GetLOC_Statement))
    (bind _out_code_2 (Class|SAPODBCStatement|ExecuteBatch (LocalVariables|GetLOC_Statement)))
    (Development|PrintString _out_code_2 true true "(R=0.000000,G=0.660000,B=1.000000,A=1.000000)" 3e+01)
    (bind (_out_code_3 _returnvalue_2) (Class|SAPODBCConnection|CommitStatement (Variables|Default|GetSAP_ODBC_Connection)))
    (Development|PrintString _out_code_3 true true (Math|Color|SelectColor "(R=0.000000,G=1.000000,B=0.000000,A=1.000000)" "(R=1.000000,G=0.000000,B=0.000000,A=1.000000)" _returnvalue_2) 3e+01)
    (return)
    (else
      (return))))